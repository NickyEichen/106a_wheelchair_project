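; Physics-driven powered chair pawn with differential front-wheel drive, an adjustable camera and a toggleable HUD.
; Each Tick mixes acceleration and turn inputs into wheel torques, or applies LeftTorque/RightTorque when ManualMode is off.
; Wheel constraints brake through angular swing drive at zero torque, and a wheel angular-velocity cap limits speed.
; Tick also derives simulated sensor state from physics: chair speed, motor RPM, wheel odometry and body-frame IMU data.
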(event `InputAxis|Max Movement`
  (params (AxisValue :type "Float (single-precision)"))
  ;[1 1 1] Increase / Decrease Torque with Q/E
  (if (> (`KismetMathLibrary.Abs` AxisValue) 0.1)
    (set `self.Drive Torque` (`KismetMathLibrary.FClamp` (+ (`self.Drive Torque`) (* AxisValue (`self.TorquePerGear`))) (`self.Min Drive Torque`) (`self.Max Drive Torque`)))
    ;[1 1 1] Display current torque on  screen
    (`KismetSystemLibrary.PrintString` (`KismetTextLibrary.Conv_TextToString` (`|FormatText` "Current Drive Torque: {torque} Nm" (`self.Drive Torque`))) true true (struct :`G` 0.020103 :`B` 1.0 :`A` 1.0) 1.0)))

(event `self.ReceiveTick`
  (params (DeltaSeconds :type "Float (single-precision)"))
  (bind _manualmode (`self.ManualMode`))
  ;[1 1 1] Drive Controls
  (`self.Update Chair State Variables` DeltaSeconds)
  (bind (_forward_torque _turning_torque) (`self.Compute Forward and Turning Torques`))
  (bind (_right_motor_torque _left_motor_torque) (`self.Compute Right and Left Motor Torques` _forward_torque _turning_torque))
  (bind _returnvalue (select `bool` _manualmode :`false` (`self.RightTorque`) :`true` _right_motor_torque))
  ;[1 1 1] Apply the torque to the wheels
  (`PrimitiveComponent.AddTorqueInRadians` (`self.WheelFR`) _returnvalue "None" true)
  (bind _returnvalue_2 (select `bool` _manualmode :`false` (`self.LeftTorque`) :`true` _left_motor_torque))
  (`PrimitiveComponent.AddTorqueInRadians` (`self.WheelFL`) _returnvalue_2 "None" true)
  ;[1 1 1] Enable / Disable Swing Drive (braking) on Front Wheel PC if their desired output torque is 0.0
  (`PhysicsConstraintComponent.SetAngularVelocityDriveTwistAndSwing` (`self.PC_WheelFR`) false (== (`KismetMathLibrary.VSize` _returnvalue) 0.0))
  (`PhysicsConstraintComponent.SetAngularVelocityDriveTwistAndSwing` (`self.PC_WheelFL`) false (== (`KismetMathLibrary.VSize` _returnvalue_2) 0.0)))

(event `self.ReceiveBeginPlay`
  (bind _brake_power (`self.Brake Power`))
  (bind _returnvalue (* (`self.Max Speed`) 44.703999))
  ;[1 1 1] Limit max speed to the configured Max Speed (mph)
  (`PrimitiveComponent.SetPhysicsMaxAngularVelocityInRadians` (`self.WheelFL`) (/ _returnvalue (`.SphereRadius` (`KismetSystemLibrary.GetComponentBounds` (`self.WheelFR`)))) false "None")
  (`PrimitiveComponent.SetPhysicsMaxAngularVelocityInRadians` (`self.WheelFR`) (/ _returnvalue (`.SphereRadius` (`KismetSystemLibrary.GetComponentBounds` (`self.WheelFR`)))) false "None")
  (`PrimitiveComponent.SetPhysicsMaxAngularVelocityInRadians` (`self.WheelRR`) (/ _returnvalue (`.SphereRadius` (`KismetSystemLibrary.GetComponentBounds` (`self.WheelRL`)))) false "None")
  (`PrimitiveComponent.SetPhysicsMaxAngularVelocityInRadians` (`self.WheelRL`) (/ _returnvalue (`.SphereRadius` (`KismetSystemLibrary.GetComponentBounds` (`self.WheelRL`)))) false "None")
  ;[1 1 1] Set brake power on the front motors
  (`PhysicsConstraintComponent.SetAngularDriveParams` (`self.PC_WheelFR`) 0.0 _brake_power 0.0)
  (`PhysicsConstraintComponent.SetAngularDriveParams` (`self.PC_WheelFL`) 0.0 _brake_power 0.0)
  ;[1 1 1] Create HUD
  (bind _returnvalue_2 (`|CreateWidget` "/Game/Blueprints/W_HUD.W_HUD_C"))
  (bind _output_get (set `self.TempHUD` _returnvalue_2))
  (`UserWidget.AddToViewport` _output_get 0))

(event `InputAxis|Camera Pan`
  (params (AxisValue :type "Float (single-precision)"))
  ;[1 1 1] Pitch / Yaw Control Over Camera
  (if (> (`KismetMathLibrary.Abs` AxisValue) 0.1)
    (`self.AddControllerYawInput` AxisValue)))

(event `InputAxis|Camera Zoom`
  (params (AxisValue :type "Float (single-precision)"))
  ;[1 1 1] Zoom Control Over camera with mouse scroll / and buttons
  (`self.Increase / Decrease Camera Zoom` AxisValue))

(event `InputAxis|Camera Tilt`
  (params (AxisValue :type "Float (single-precision)"))
  ;[1 1 1] Pitch / Yaw Control Over Camera
  (if (> (`KismetMathLibrary.Abs` AxisValue) 0.1)
    (`self.AddControllerPitchInput` AxisValue)))

(event `InputAxis|PinchZoom`
  (params (AxisValue :type "Float (single-precision)"))
  (bind _pinch_value (`self.Pinch Value`))
  ;[1 1 1] Pinch Zooming on Touchscreens
  (if (not (== AxisValue _pinch_value))
    (`/Engine/EditorBlueprintResources/StandardMacros.CompareFloat` AxisValue _pinch_value
      (:`>`
        (`self.Increase / Decrease Camera Zoom` (* (`self.Pinch Scale`) (- (`KismetMathLibrary.FClamp` (/ _pinch_value AxisValue)) 1.0))))
      (:`<`
        (`self.Increase / Decrease Camera Zoom` (* (- 1.0 (`KismetMathLibrary.FClamp` (/ AxisValue _pinch_value))) (`self.Pinch Scale`)))))
    (set `self.Pinch Value` AxisValue)))

(event `Key|H`
  (params (Key :type "Key Structure"))
  ;[1 1 1] Toggle HUD Visibility When Pressing "H" Key
  (:`Pressed`
    (if (`Widget.IsVisible` (`self.TempHUD`))
      (`Widget.SetVisibility` (`self.TempHUD`) "Collapsed")
      (else
        (`Widget.SetVisibility` (`self.TempHUD`) "Visible")))))

(event `Key|Gesture_Pinch`
  (params (Key :type "Key Structure"))
  ;[1 1 1] Pinch Zooming on Touchscreens
  ;;[1 1 1] Make sure to set the Pinch Value to 1.0 every time the user starts touching the screen
  (:`Pressed`
    (`/Engine/EditorBlueprintResources/StandardMacros.DoOnce` false :!label _label
      (:`Completed`
        (set `self.Pinch Value` 1.0))))
  (:`Released`
    (goto _label :!via `Reset`)))

(fn `Compute Forward and Turning Torques`
  (returns (`Forward Torque` :type "Float (double-precision)") (`Turning Torque` :type "Float (double-precision)"))
  (locals (_forward :type "Float (double-precision)" :default 0.0) (_turning :type "Float (double-precision)" :default 0.0))
  (bind _returnvalue (`self.GetInputAxisValue`))
  (bind _returnvalue_2 (`self.GetInputAxisValue`))
  (bind _drive_torque (`self.Drive Torque`))
  (if (< (`KismetMathLibrary.Abs` _returnvalue_2) 0.05)
    (set `local._forward` 0.0)
    (else
      (set `local._forward` (* _returnvalue_2 _drive_torque))))
  (if (< (`KismetMathLibrary.Abs` _returnvalue) 0.05)
    (set `local._turning` 0.0)
    (else
      (set `local._turning` (* (* _drive_torque (`self.Turn Torque Factor`)) _returnvalue))))
  (return (`local._forward`) (`local._turning`)))

(fn `Compute Right and Left Motor Torques`
  (params (`Forward Torque` :type "Float (double-precision)") (`Turning Torque` :type "Float (double-precision)"))
  (returns (`Right Motor Torque` :type "Vector Structure") (`Left Motor Torque` :type "Vector Structure"))
  (locals (NewLocalVar_0 :type "Float (double-precision)" :default 0.0) (NewLocalVar_1 :type "Float (double-precision)" :default 0.0))
  (return (* (`SceneComponent.GetRightVector` (`self.WheelFR`)) (* (+ `Forward Torque` (* `Turning Torque` -1.0)) -1.0)) (* (`SceneComponent.GetRightVector` (`self.WheelFL`)) (+ `Forward Torque` `Turning Torque`))))

(fn `Get Motor RPM`
  (params (Wheel :type "StaticMeshComponent Object Reference") (`Reverse Direction` :type "Float (double-precision)" :default 1.0))
  (returns (RPM :type "Float (double-precision)"))
  (bind _returnvalue (`SceneComponent.GetRightVector` Wheel))
  (bind _returnvalue_2 (`KismetMathLibrary.Dot_VectorVector` (`PrimitiveComponent.GetPhysicsAngularVelocityInRadians` Wheel "None") _returnvalue))
  (return (* (* (/ (* (`KismetMathLibrary.SignOfFloat` _returnvalue_2) (`KismetMathLibrary.VSize` (* (/ _returnvalue (`KismetMathLibrary.VSize` _returnvalue)) _returnvalue_2))) 6.283184) 60.0) `Reverse Direction`)))

(fn `Get Motor Speed`
  (params (Wheel :type "StaticMeshComponent Object Reference") (`Reverse Direction` :type "Float (double-precision)" :default 1.0))
  (returns (Speed :type "Float (double-precision)"))
  (bind _returnvalue (`SceneComponent.GetRightVector` Wheel))
  (bind _returnvalue_2 (`KismetMathLibrary.Dot_VectorVector` (`PrimitiveComponent.GetPhysicsAngularVelocityInRadians` Wheel "None") _returnvalue))
  (return (* (/ (* (`.SphereRadius` (`KismetSystemLibrary.GetComponentBounds` Wheel)) (* (`KismetMathLibrary.SignOfFloat` _returnvalue_2) (`KismetMathLibrary.VSize` (* (/ _returnvalue (`KismetMathLibrary.VSize` _returnvalue)) _returnvalue_2)))) 100.0) `Reverse Direction`)))

(fn `Increase / Decrease Camera Zoom`
  (params (`Axis Value` :type "Float (double-precision)"))
  (if (> (`KismetMathLibrary.Abs` `Axis Value`) 0.1)
    (set `SpringArmComponent.TargetArmLength` (`KismetMathLibrary.FClamp` (+ (* `Axis Value` (`self.Zoom Speed`)) (`SpringArmComponent.TargetArmLength` (`self.SpringArm`))) (`self.Min Camera Distance`) (`self.Max Camera Distance`)) (`self.SpringArm`))))

(fn `Update Chair State Variables`
  (params (`Delta Seconds` :type "Float (double-precision)"))
  (bind _wheelfl (`self.WheelFL`))
  (bind _wheelfr (`self.WheelFR`))
  (bind _body (`self.Body`))
  (`|ExecutionSequence`
    (:`then_0`
      ;[1 1 1] Chair Forward Speed Update
      (bind _returnvalue (`PrimitiveComponent.GetPhysicsLinearVelocity` _body "None"))
      (set `self.ChairSpeed` (* (/ (`KismetMathLibrary.Dot_VectorVector` _returnvalue (`SceneComponent.GetForwardVector` _body)) 100.0) 2.23694)))
    (:`then_1`
      (`self.Update IMU Data` `Delta Seconds`))
    (:`then_2`
      ;[1 1 1] Right Motor (Front Wheel) Speed / RPM Update
      (bind _rpm (`self.Get Motor RPM` _wheelfr -1.0))
      (set `self.WheelFR_RPM` _rpm)
      (set `self.WheelFRSpeed` (`KismetMathLibrary.Dot_VectorVector` (`PrimitiveComponent.GetPhysicsAngularVelocityInDegrees` _wheelfr "None") (`SceneComponent.GetRightVector` _wheelfr))))
    (:`then_3`
      ;[1 1 1] Left Motor (Front Wheel) Speed / RPM Update
      (bind _rpm_2 (`self.Get Motor RPM` _wheelfl))
      (set `self.WheelFL_RPM` _rpm_2)
      (set `self.WheelFLSpeed` (`KismetMathLibrary.Dot_VectorVector` (`PrimitiveComponent.GetPhysicsAngularVelocityInDegrees` _wheelfl "None") (`SceneComponent.GetRightVector` _wheelfl))))
    (:`then_4`
      ;[1 1 1] Update Front Right Wheel Odometry
      (bind _speed (`self.Get Motor Speed` (`self.WheelFR`) -1.0))
      (if (> (`KismetMathLibrary.Abs` _speed) 0.05)
        (set `self.WheelFROdometry` (+ (* _speed `Delta Seconds`) (`self.WheelFROdometry`)))))
    (:`then_5`
      ;[1 1 1] Update Front Left Wheel Odometry
      (bind _speed_2 (`self.Get Motor Speed` (`self.WheelFL`)))
      (if (> (`KismetMathLibrary.Abs` _speed_2) 0.05)
        (set `self.WheelFLOdometry` (+ (* _speed_2 `Delta Seconds`) (`self.WheelFLOdometry`)))))))

(fn `Update IMU Data`
  (params (`Delta Seconds` :type "Float (double-precision)"))
  (bind _body (`self.Body`))
  (`|ExecutionSequence`
    (:`then_0`
      (set `self.AngularVelocity` (`KismetMathLibrary.LessLess_VectorRotator` (`PrimitiveComponent.GetPhysicsAngularVelocityInDegrees` _body "None") (`SceneComponent.K2_GetComponentRotation` _body))))
    (:`then_1`
      (bind _returnvalue (`PrimitiveComponent.GetPhysicsLinearVelocity` _body "None"))
      (bind _returnvalue_2 (/ (`KismetMathLibrary.LessLess_VectorRotator` _returnvalue (`SceneComponent.K2_GetComponentRotation` _body)) 100.0))
      (set `self.LinearAcceleration` (/ (- _returnvalue_2 (`self.LinearVelocity`)) `Delta Seconds`))
      (set `self.LinearVelocity` _returnvalue_2))))

(fn `UserConstructionScript`)